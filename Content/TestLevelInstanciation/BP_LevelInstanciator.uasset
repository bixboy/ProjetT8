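; BP_LevelInstanciator is an actor that swaps level instances in step with the wave flow.
; On BeginPlay it binds to BP_WaveManager's begin-wave and start-buff-choice dispatchers.
; Each wave's level loads as a level instance at the actor's location, under a fixed override name.
; When buff choice starts, it passes that level to BP_LevelTest's animation component to play the end animation rather than unloading it directly.
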(event `self.ReceiveBeginPlay`
  (bind _returnvalue (`GameplayStatics.GetActorOfClass` "/Game/BP_/WaveManagement/BP_WaveManager.BP_WaveManager_C"))
  (`/Engine/EditorBlueprintResources/StandardMacros.IsValid` _returnvalue
    (:`Is Valid`
      (add `/Game/BP_/WaveManagement/BP_WaveManager.ED_BeginWave` _returnvalue (delegate `ED_BeginWave_Event_0`))
      (add `/Game/BP_/WaveManagement/BP_WaveManager.ED_StartBuffChoice` _returnvalue (delegate `ED_StartBuffChoice_Event`)))
    (:`Is Not Valid`
      (`KismetSystemLibrary.PrintString` "not valid wave manager"))))

(event `ED_StartBuffChoice_Event`
  (`self.CE_UnloadLevel`))

(event `ED_BeginWave_Event_0`
  (params (Wave :type "/Game/BP_/WaveManagement/WaveData Structure"))
  (`self.CE_InstaciateLevel` Wave_Level_15_CCF14410461F9EF8ACDFA8A41108DE19))

(event `CE_InstaciateLevel`
  (params (Level :type String))
  (bind (_boutsuccess _returnvalue) (`LevelStreamingDynamic.LoadLevelInstance` Level (`self.K2_GetActorLocation`) (struct) "InstanciatedLevel" null))
  (set `self.Level` _returnvalue))

(event `CE_UnloadLevel`
  (bind _returnvalue (`GameplayStatics.GetActorOfClass` "/Game/TestLevelInstanciation/BP_LevelTest.BP_LevelTest_C"))
  (`/Engine/EditorBlueprintResources/StandardMacros.IsValid` _returnvalue
    (:`Is Valid`
      (set `self.LevelBP` _returnvalue)
      (`/Game/TestLevelInstanciation/AC_LevelAnimation.CE_InitEndAnim` (`/Game/TestLevelInstanciation/BP_LevelTest.AC_LevelAnimation` (`self.LevelBP`)) (`self.Level`)))
    (:`Is Not Valid`
      (`KismetSystemLibrary.PrintString` "NoLevel in scene"))))

(fn `UserConstructionScript`)