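; Actor component that animates a level's static meshes rising in and sinking out as battle waves start and end.
; BeginPlay stores each mesh's Z and drops it below ground, then after a delay recursive events move meshes back in reverse order over random durations.
; It then tells BP_WaveManager to start the battle.
; The end animation lowers the meshes, sets CanEndWave and requests unload of the passed level instance.
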(event `self.ReceiveBeginPlay`
  (bind _output_get (set `self.Meshes` (`Actor.K2_GetComponentsByClass` (`self.GetOwner`) "/Script/Engine.StaticMeshComponent")))
  (bind _output_get_2 (set `self.NbMesh` (`KismetArrayLibrary.Array_Length` _output_get)))
  (`/Engine/EditorBlueprintResources/StandardMacros.DecrementInt` _output_get_2
    (:`  `
      (for _array_element (`self.Meshes`)
        (bind (_relativelocation_x _relativelocation_y _relativelocation_z) (`KismetMathLibrary.BreakVector` (`SceneComponent.RelativeLocation` _array_element)))
        (`KismetArrayLibrary.Array_Add` (`self.Zpos`) _relativelocation_z)
        (`SceneComponent.K2_SetRelativeLocation` _array_element (`KismetMathLibrary.MakeVector` _relativelocation_x _relativelocation_y (- (+ (* (.z (`.BoxExtent` (`KismetSystemLibrary.GetComponentBounds` _array_element))) -2.0) -20.0) _relativelocation_z)) false false)
        (bind _returnvalue (`GameplayStatics.GetActorOfClass` "/Game/BP_/WaveManagement/BP_WaveManager.BP_WaveManager_C"))
        (set `self.WaveManager` _returnvalue))
      (`KismetSystemLibrary.Delay` 1.0)
      (`self.CE_PlaySpawnAnim`))))

(event `CE_PlaySpawnAnim`
  (bind _nbmesh (`self.NbMesh`))
  (bind _output (`|GetArrayItem` (`self.Meshes`) _nbmesh))
  (bind (_relativelocation_x _relativelocation_y) (`KismetMathLibrary.BreakVector` (`SceneComponent.RelativeLocation` _output)))
  (if (>= (`self.NbMesh`) 0)
    (`KismetSystemLibrary.MoveComponentTo` _output (`KismetMathLibrary.MakeVector` _relativelocation_x _relativelocation_y (`|GetArrayItem` (`self.Zpos`) _nbmesh)) (`SceneComponent.RelativeRotation` _output) false false (`KismetMathLibrary.RandomFloat`))
    (`/Engine/EditorBlueprintResources/StandardMacros.DecrementInt` (`self.NbMesh`)
      (:`  `
        (`self.CE_PlaySpawnAnim`)))
    (else
      (`/Game/BP_/WaveManagement/BP_WaveManager.CE_StartBattle` (`self.WaveManager`)))))

(event `CE_InitEndAnim`
  (params (Level :type "LevelStreamingDynamic Object Reference"))
  (bind _output_get (set `self.NbMesh` (`KismetArrayLibrary.Array_Length` (`self.Meshes`))))
  (`/Engine/EditorBlueprintResources/StandardMacros.DecrementInt` _output_get
    (:`  `
      (set `self.Level` Level)
      (`self.CE_PlayDeSpawnAnim`))))

(event `CE_PlayDeSpawnAnim`
  (bind _output (`|GetArrayItem` (`self.Meshes`) (`self.NbMesh`)))
  (bind (_relativelocation_x _relativelocation_y) (`KismetMathLibrary.BreakVector` (`SceneComponent.RelativeLocation` _output)))
  (if (>= (`self.NbMesh`) 0)
    (`KismetSystemLibrary.MoveComponentTo` _output (`KismetMathLibrary.MakeVector` _relativelocation_x _relativelocation_y -500.0) (`SceneComponent.RelativeRotation` _output) false false (/ (`KismetMathLibrary.RandomFloat`) 2.0))
    (`/Engine/EditorBlueprintResources/StandardMacros.DecrementInt` (`self.NbMesh`)
      (:`  `
        (`self.CE_PlayDeSpawnAnim`)))
    (else
      (set `/Game/BP_/WaveManagement/BP_WaveManager.CanEndWave` true (`self.WaveManager`))
      (`LevelStreaming.SetIsRequestingUnloadAndRemoval` (`self.Level`) true))))