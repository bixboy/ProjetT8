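; Enemy minion Blueprint whose look and damage vary with a difficulty level.
; The CESpawn event takes a Difficulty index, applies the matching entry from Materials to mesh slot 3, and multiplies Damage by Difficulty plus one.
; The construction script only calls its parent, and the BeginPlay node is disabled.
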(event `self.CE_Spawn`
  (params (Difficulty :type Integer))
  (`PrimitiveComponent.SetMaterial` (`self.Mesh`) 3 (`|GetArrayItem` (`self.Materials`) Difficulty))
  (set `self.Damage` (* (`self.Damage`) (+ Difficulty 1))))

(fn `UserConstructionScript`
  (`parent.UserConstructionScript`))