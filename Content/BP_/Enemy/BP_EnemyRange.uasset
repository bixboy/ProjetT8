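; BP_EnemyRange is a ranged enemy that shoots projectiles at the player.
; Every tick it yaws to face the player's mesh.
; Its Attack event spawns a gravity-free BP_ProjectileEnemy at the ShootPoint socket, rotated along the line from its own location to the player.
; On spawn, a Difficulty index picks its material and, plus one, multiplies damage, max health, walk speed and projectile speed.
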(event `self.ReceiveTick`
  (params (DeltaSeconds :type "Float (single-precision)"))
  (bind (_returnvalue_roll _returnvalue_pitch _returnvalue_yaw) (`KismetMathLibrary.BreakRotator` (`KismetMathLibrary.FindLookAtRotation` (`self.K2_GetActorLocation`) (`SceneComponent.K2_GetComponentLocation` (`Character.Mesh` (`GameplayStatics.GetPlayerCharacter` 0))))))
  (`self.K2_SetActorRotation` (`KismetMathLibrary.MakeRotator` 0.0 0.0 _returnvalue_yaw)))

(event `/Game/BP_/Interface/BPI_EnemyAI.Attack`
  (`|SpawnActorFromClass` "/Game/BP_/Weapons/BP_ProjectileEnemy.BP_ProjectileEnemy_C" (`KismetMathLibrary.MakeTransform` (`SceneComponent.GetSocketLocation` (`self.Mesh`) "ShootPoint") (`KismetMathLibrary.FindLookAtRotation` (`self.K2_GetActorLocation`) (`self.K2_GetActorLocation` (`GameplayStatics.GetPlayerCharacter` 0))) (0.5 0.5 0.5)) "Undefined" "MultiplyWithRoot" null (`self.Damage`) (`self.ProjectilVelocity`) 0.0 null))

(event `self.CE_Spawn`
  (params (Difficulty :type Integer))
  (bind _returnvalue (+ Difficulty 1))
  (`PrimitiveComponent.SetMaterial` (`self.Mesh`) 3 (`|GetArrayItem` (`self.Materials`) Difficulty))
  (set `self.Damage` (* (`self.Damage`) _returnvalue))
  (set `/Game/BP_/ActorComponent/Health/BPC_Health.MaxHealth` (* _returnvalue (`/Game/BP_/ActorComponent/Health/BPC_Health.MaxHealth` (`self.BPC_Health`))) (`self.BPC_Health`))
  (set `CharacterMovementComponent.MaxWalkSpeed` (* _returnvalue (`CharacterMovementComponent.MaxWalkSpeed` (`self.CharacterMovement`))) (`self.CharacterMovement`))
  (set `self.ProjectilVelocity` (* _returnvalue (`self.ProjectilVelocity`))))

(fn `UserConstructionScript`
  (`parent.UserConstructionScript`))