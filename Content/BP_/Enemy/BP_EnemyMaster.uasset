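; Base enemy actor that other enemies derive from, handling attacks on the player and its own death.
; On BeginPlay it caches the first-person player character, and Attack deals its damage through that character's health component.
; Incoming damage goes to its own health component, and a true result fires the OnDestroy dispatcher and destroys the actor.
; CE_Spawn takes a difficulty but is empty here.
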(event `self.ReceiveBeginPlay`
  (bind _asbp_first_person_character (cast `/Game/FirstPerson/Blueprints/BP_FirstPersonCharacter` (`GameplayStatics.GetPlayerCharacter` 0)))
  (set `self.Player` _asbp_first_person_character))

(event `/Game/BP_/Interface/BPI_Attack.Attack`
  (`/Game/BP_/ActorComponent/Health/BPC_Health.TakeDamage` (`/Game/FirstPerson/Blueprints/BP_FirstPersonCharacter.BPC_Health` (`self.Player`)) false (`self.Damage`) "None"))

(event `/Game/BP_/Interface/BPI_TakeDamage.TakeDamage`
  (params (Damage :type "Float (double-precision)") (BoneName :type Name))
  (bind _isdead (`/Game/BP_/ActorComponent/Health/BPC_Health.TakeDamage` (`self.BPC_Health`) false Damage BoneName))
  (if _isdead
    (`self.ED_OnDestroy`)
    (`self.K2_DestroyActor`)))

(event `CE_Spawn`
  (params (Difficulty :type Integer)))

(fn `UserConstructionScript`)