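; BP_Lava is a lava hazard that damages the first-person player while they stand inside its Box volume.
; BeginPlay caches the player character and plays the lava loop sound at the world origin.
; Box overlap sets DoDamage and starts a self-calling, one-second Delay loop that hurts the player's BPCHealth component and plays a damage sound at their location.
; End overlap clears the flag, ending the loop, which then resets it to true.
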(event `self.ReceiveBeginPlay`
  (bind _asbp_first_person_character (cast `/Game/BP_/BP_Player/BP_FirstPersonCharacter` (`GameplayStatics.GetPlayerCharacter` 0)))
  (set `self.Player` _asbp_first_person_character)
  (`GameplayStatics.PlaySoundAtLocation` null (0.0 0.0 0.0) (struct) 1.0 1.0 0.0 null null null null) ; Lava Loop
)

(event `self.Box.OnComponentBeginOverlap`
  (params (OverlappedComponent :type "PrimitiveComponent Object Reference") (OtherActor :type "Actor Object Reference") (OtherComp :type "PrimitiveComponent Object Reference") (OtherBodyIndex :type Integer) (bFromSweep :type Boolean) (SweepResult :type "HitResult Structure (by ref)"))
  (cast `/Game/BP_/BP_Player/BP_FirstPersonCharacter` OtherActor)
  (set `self.DoDamage` true)
  (`self.CE_DealDamage`)
  (`KismetSystemLibrary.PrintString` "Overlapped"))

(event `CE_DealDamage`
  (if (`self.DoDamage`)
    (`/Game/BP_/ActorComponent/Health/BPC_Health.TakeDamage` (`/Game/BP_/BP_Player/BP_FirstPersonCharacter.BPC_Health` (`self.Player`)) false (`self.Damages`) "None" (0.0 0.0 0.0))
    (`GameplayStatics.PlaySoundAtLocation` null (`self.K2_GetActorLocation` (`GameplayStatics.GetPlayerCharacter` 0)) (struct) 1.0 1.0 0.0 null null null null) ; LavaDamage Sound
    (`KismetSystemLibrary.Delay` 1.0)
    (`self.CE_DealDamage`)
    (else
      (set `self.DoDamage` true))))

(event `self.Box.OnComponentEndOverlap`
  (params (OverlappedComponent :type "PrimitiveComponent Object Reference") (OtherActor :type "Actor Object Reference") (OtherComp :type "PrimitiveComponent Object Reference") (OtherBodyIndex :type Integer))
  (cast `/Game/BP_/BP_Player/BP_FirstPersonCharacter` OtherActor)
  (set `self.DoDamage` false)
  (`KismetSystemLibrary.PrintString` "Stop Overlap"))

(fn `UserConstructionScript`)