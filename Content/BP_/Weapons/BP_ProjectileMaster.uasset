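; BP_ProjectileMaster is a weapon projectile, named as a master class, that deals damage on hit.
; Its construction script feeds the Speed and Gravity variables into the ProjectileMovement component.
; On hit, it triggers BPC_Blood effects if the target has that component.
; Targets implementing BPI_TakeDamage receive damage with the hit bone name, and only then does it spawn dust and destroy itself.
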(event `self.ReceiveHit`
  (params (MyComp :type "PrimitiveComponent Object Reference") (Other :type "Actor Object Reference") (OtherComp :type "PrimitiveComponent Object Reference") (bSelfMoved :type Boolean) (HitLocation :type "Vector Structure") (HitNormal :type "Vector Structure") (NormalImpulse :type "Vector Structure") (Hit :type "HitResult Structure (by ref)"))
  (bind _returnvalue (`self.GetComponentByClass` Other "/Game/BP_/ActorComponent/Blood/BPC_Blood.BPC_Blood_C"))
  (`/Engine/EditorBlueprintResources/StandardMacros.IsValid` _returnvalue
    (:`Is Valid`
      (`/Game/BP_/ActorComponent/Blood/BPC_Blood.BloodEffect` _returnvalue HitLocation HitNormal))
    (:`Is Not Valid`
      _))
  (if (`KismetSystemLibrary.DoesImplementInterface` Other "/Game/BP_/Interface/BPI_TakeDamage.BPI_TakeDamage_C")
    (message `/Game/BP_/Interface/BPI_TakeDamage.TakeDamage` Other (`self.Damage`) (`.HitBoneName` (`GameplayStatics.BreakHitResult` Hit)))
    (`GameplayStatics.SpawnEmitterAtLocation` "/Game/StarterContent/Particles/P_Ambient_Dust.P_Ambient_Dust" HitLocation)
    (`self.K2_DestroyActor`)))

(fn `UserConstructionScript`
  (bind _projectilemovement (`self.ProjectileMovement`))
  (set `ProjectileMovementComponent.InitialSpeed` (`self.Speed`) _projectilemovement)
  (set `ProjectileMovementComponent.MaxSpeed` (`self.Speed`) _projectilemovement)
  (set `ProjectileMovementComponent.ProjectileGravityScale` (`self.Gravity`) _projectilemovement))