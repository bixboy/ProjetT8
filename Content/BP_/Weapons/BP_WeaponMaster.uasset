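; Base weapon actor for the first-person player, handling equip, attack and unequip through montages.
; StartEquipWeapons attaches it to the SwordGrip socket and plays the equip montage; unequip destroys the actor once its montage completes.
; FireStarted stores close damage and attack speed via Attack, plays a swipe sound and montage, and blocks further attacks until the montage completes.
; SecondAttack is an empty stub, and range damage is unused.
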(event `self.ReceiveBeginPlay`
  (bind _asbp_first_person_character (cast `/Game/BP_/BP_Player/BP_FirstPersonCharacter` (`GameplayStatics.GetPlayerCharacter` 0)))
  (set `self.Player` _asbp_first_person_character))

(event `/Game/BP_/Interface/BPI_Weapon.FireStarted`
  (params (PlayerCloseDamage :type "Float (double-precision)") (PlayerRangeDamage :type "Float (double-precision)") (PlayerFireRate :type "Float (double-precision)"))
  (if (`self.CanAttack`)
    (set `self.CanAttack` false)
    (`self.Attack` PlayerCloseDamage PlayerRangeDamage PlayerFireRate)
    (`GameplayStatics.PlaySoundAtLocation` "/Game/BP_/Sounds/Sword/A_SwordSwipe.A_SwordSwipe" (`SceneComponent.K2_GetComponentLocation` (`self.Weapon`)) (struct) 1.0 1.0 0.0 null null null null)
    (`|PlayMontage` (`/Game/BP_/BP_Player/BP_FirstPersonCharacter.FirstPersonMesh` (`self.Player`)) (`self.AnimAttack`) (`self.SpeedAnim`)
      (:`OnCompleted`
        (set `self.CanAttack` true)))))

(event `UnEquipWeapon`
  (params (SkeletalMesh :type "SkeletalMeshComponent Object Reference") (AnimSpeed :type "Float (double-precision)"))
  (`|PlayMontage` SkeletalMesh (`self.AnimUnequip`) AnimSpeed
    (:`OnCompleted`
      (`self.K2_DestroyActor`))))

(event `EquipWeapon`
  (params (SkeletalMes :type "SkeletalMeshComponent Object Reference") (AnimSpeed :type "Float (double-precision)"))
  (`|PlayMontage` SkeletalMes (`self.AnimEquip`) AnimSpeed))

(fn `Attack`
  (params (PlayerCloseDamage :type "Float (double-precision)") (PlayerRangeDamage :type "Float (double-precision)") (PlayerFireRate :type "Float (double-precision)"))
  (set `self.Damage` PlayerCloseDamage)
  (set `self.AttackSpeed` PlayerFireRate))

(fn `SecondAttack`
  (params (PlayerRangeDamage :type "Float (double-precision)") (PlayerFireRate :type "Float (double-precision)") (Range :type "Float (double-precision)") (NbProjectiles :type Integer))
  (if (`self.HaveSecondAttack`)
    _))

(fn `StartEquipWeapons`
  (params (PlayerSkeletalMesh :type "SkeletalMeshComponent Object Reference") (SkeletalMesh :type "SkeletalMeshComponent Object Reference") (AnimSpeed :type "Float (double-precision)"))
  (returns (CurrentWeapon :type "/Game/BP_/Weapons/BP_WeaponMaster Object Reference"))
  (`self.K2_AttachToComponent` PlayerSkeletalMesh "SwordGrip" "KeepRelative" "KeepRelative" "KeepRelative")
  (`self.EquipWeapon` (`local.SkeletalMesh`) (`local.AnimSpeed`))
  (return self))

(fn `UserConstructionScript`)