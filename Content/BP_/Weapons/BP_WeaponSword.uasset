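; Sword weapon Blueprint that deals fixed melee damage through sphere traces between the mesh's Start and End sockets.
; Start/StopSwordTrace run a fast looping timer that calls SwordTrace, ignoring the player.
; A hit clears CanHit; actors with BPC_Blood get blood effects, and those also implementing BPI_TakeDamage receive damage with bone name plus camera shake.
; Only that damage path re-arms CanHit and its DoOnce, after a short delay.
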(event `/Game/BP_/Interface/BPI_Weapon.StartSwordTrace`
  ;[0.05729 0.05729 0.05729] Sword Trace
  (bind _returnvalue (`KismetSystemLibrary.K2_SetTimerDelegate` (delegate `SwordTraceLoop`) 0.001 true))
  (set `self.SwordTraceEvent` _returnvalue))

(event `/Game/BP_/Interface/BPI_Weapon.StopSwordTrace`
  ;[0.05729 0.05729 0.05729] Sword Trace
  (`KismetSystemLibrary.K2_ClearAndInvalidateTimerHandle` (`self.SwordTraceEvent`)))

(event `SwordTraceLoop`
  ;[0.05729 0.05729 0.05729] Sword Trace
  (bind (_hitenemy _actor _bonesname) (`self.SwordTrace`))
  (if _hitenemy
    (`/Engine/EditorBlueprintResources/StandardMacros.DoOnce` false :!label _label
      (:`Completed`
        (message `/Game/BP_/Interface/BPI_TakeDamage.TakeDamage` _actor 30.0 _bonesname)
        (`GameplayStatics.PlayWorldCameraShake` "/Game/BP_/Camera/BP_CameraShakeSwordAttack.BP_CameraShakeSwordAttack_C" (0.0 0.0 0.0) 0.0 2000.0)
        (`KismetSystemLibrary.Delay` 0.5)
        (set `self.CanHit` true)
        (goto _label :!via `Reset`)))))

(fn `Attack`
  (params (PlayerCloseDamage :type "Float (double-precision)") (PlayerRangeDamage :type "Float (double-precision)") (PlayerFireRate :type "Float (double-precision)"))
  (`parent.Attack` PlayerCloseDamage PlayerRangeDamage PlayerFireRate))

(fn `SwordTrace`
  (returns (HitEnemy :type Boolean) (Actor :type "Actor Object Reference") (BonesName :type Name))
  (bind _weapon (`self.Weapon`))
  (if (`self.CanHit`)
    (bind (_outhit _returnvalue) (`KismetSystemLibrary.SphereTraceSingle` (`SceneComponent.GetSocketLocation` _weapon "Start") (`SceneComponent.GetSocketLocation` _weapon "End") 12.0 "TraceTypeQuery1" false (`|MakeArray` (`GameplayStatics.GetPlayerCharacter` 0) :!type "Actor Object Reference") "None" true (struct :`R` 1.0 :`A` 1.0) (struct :`G` 1.0 :`A` 1.0) 0.5))
    (if _returnvalue
      (set `self.CanHit` false)
      (bind (_bblockinghit _binitialoverlap _time _distance _location _impactpoint _normal _impactnormal _physmat _hitactor _hitcomponent _hitbonename) (`GameplayStatics.BreakHitResult` _outhit))
      (bind _returnvalue_2 (`self.GetComponentByClass` _hitactor "/Game/BP_/ActorComponent/Blood/BPC_Blood.BPC_Blood_C"))
      (`/Engine/EditorBlueprintResources/StandardMacros.IsValid` _returnvalue_2
        (:`Is Valid`
          (`/Game/BP_/ActorComponent/Blood/BPC_Blood.BloodEffect` _returnvalue_2 _impactpoint _impactnormal)
          (if (`KismetSystemLibrary.DoesImplementInterface` _hitactor "/Game/BP_/Interface/BPI_TakeDamage.BPI_TakeDamage_C")
            (return true _hitactor _hitbonename)
            (else
              (return false null "None"))))))))

(fn `UserConstructionScript`
  (`parent.UserConstructionScript`))