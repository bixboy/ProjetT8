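; BP_LaserBeam is a short-lived laser weapon effect that deals hitscan damage from the player's camera.
; StartLaser line-traces to Range, points the Niagara beam at the impact or trace end, and plays impact sound at the player's location on hits.
; Actors implementing BPI_TakeDamage get a BPC_Blood effect and damage with bone and normal.
; After one second, StopLaser deactivates both effects, animates beam scale by timeline, then destroys the actor.
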(event `self.ReceiveBeginPlay`
  (bind _asbp_first_person_character (cast `/Game/BP_/BP_Player/BP_FirstPersonCharacter` (`GameplayStatics.GetPlayerCharacter` 0)))
  (set `self.Player` _asbp_first_person_character))

(event `StartLaser`
  (bind _firstpersoncamera (`/Game/BP_/BP_Player/BP_FirstPersonCharacter.FirstPersonCamera` (`self.Player`)))
  (bind _returnvalue (`SceneComponent.K2_GetComponentLocation` _firstpersoncamera))
  (bind _outhit (`KismetSystemLibrary.LineTraceSingle` :`Start` _returnvalue :`End` (+ _returnvalue (* (`KismetMathLibrary.GetForwardVector` (`SceneComponent.K2_GetComponentRotation` _firstpersoncamera)) (`self.Range`))) :`TraceChannel` "TraceTypeQuery2" :`DrawTime` 2.0))
  (bind (_bblockinghit _binitialoverlap _time _distance _location _impactpoint _normal _impactnormal _physmat _hitactor _hitcomponent _hitbonename _bonename _hititem _elementindex _faceindex _tracestart _traceend) (`GameplayStatics.BreakHitResult` _outhit))
  (bind _returnvalue_2 (`KismetSystemLibrary.IsValid` _hitcomponent))
  (`FXSystemComponent.SetVectorParameter` (`self.Laser`) "User.BeamEnd" (`KismetMathLibrary.SelectVector` _impactpoint _traceend _returnvalue_2))
  (if _returnvalue_2
    (`FXSystemComponent.SetVectorParameter` (`self.LaserHit`) "User.HitLocation" _impactpoint)
    (`GameplayStatics.PlaySoundAtLocation` "/Game/BP_/Sounds/Sword/A_ProjectileImpact.A_ProjectileImpact" (`self.K2_GetActorLocation` (`self.Player`)) (struct) 1.0 1.0 0.0 null null null null)
    (if (`KismetSystemLibrary.DoesImplementInterface` _hitactor "/Game/BP_/Interface/BPI_TakeDamage.BPI_TakeDamage_C")
      (`/Game/BP_/ActorComponent/Blood/BPC_Blood.BloodEffect` (`self.GetComponentByClass` _hitactor "/Game/BP_/ActorComponent/Blood/BPC_Blood.BPC_Blood_C") _impactpoint _impactnormal)
      (message `/Game/BP_/Interface/BPI_TakeDamage.TakeDamage` _hitactor (`self.Damage`) _hitbonename _impactnormal)))
  (`ActorComponent.Activate` (`self.LaserHit`) false)
  (`KismetSystemLibrary.Delay` 1.0)
  (`self.StopLaser`))

(event `StopLaser`
  (`/Engine/EditorBlueprintResources/StandardMacros.DoOnce` false
    (:`Completed`
      (`ActorComponent.Deactivate` (`self.Laser`))
      (`ActorComponent.Deactivate` (`self.LaserHit`))
      (bind (_direction _scale) (`Timeline|StopEffect` :!via `PlayFromStart`)
        (:`Update`
          (`FXSystemComponent.SetFloatParameter` (`self.Laser`) "User.Scale" _scale))
        (:`Finished`
          (`self.K2_DestroyActor`))))))

(fn `UserConstructionScript`)