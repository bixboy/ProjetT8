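; BPC_Health is an actor component that manages health, damage, healing and death state.
; BeginPlay fills health to maximum and caches the owner as BP_EnemyMaster if the cast succeeds.
; TakeDamage doubles Head hits and returns death state; OneShot applies only to non-head hits and skips the Death call, itself an empty stub.
; Healing refills fully or adds a clamped amount, while UpdateMaxLife scales maximum health up.
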(event `self.ReceiveBeginPlay`
  (set `self.CurrentHealth` (`self.MaxHealth`))
  (bind _asbp_enemy_master (cast `/Game/BP_/Enemy/BP_EnemyMaster` (`self.GetOwner`)))
  (set `self.As BP Enemy Master` _asbp_enemy_master))

(fn `Death`)

(fn `Healing`
  (params (RegenFullHealth :type Boolean) (`Health Regen` :type "Float (double-precision)"))
  (if RegenFullHealth
    (set `self.CurrentHealth` (`self.MaxHealth`))
    (else
      (bind _output_get (set `self.CurrentHealth` (`KismetMathLibrary.FClamp` (+ (`self.CurrentHealth`) `Health Regen`) 0.0 (`self.MaxHealth`))))
      (`KismetSystemLibrary.PrintString` (`KismetStringLibrary.Conv_DoubleToString` _output_get)))))

(fn `TakeDamage`
  (params (OneShot :type Boolean) (Damage :type "Float (double-precision)") (BoneName :type Name))
  (returns (IsDead :type Boolean))
  (if (not (== BoneName "Head"))
    (if (`local.OneShot`)
      (set `self.CurrentHealth` 0.0)
      (bind _output_get (set `self.IsDead` true))
      (return _output_get)
      (else
        (bind _output_get_2 (set `self.CurrentHealth` (- (`self.CurrentHealth`) (`local.Damage`))))))
    (else
      (set `self.CurrentHealth` (- (`self.CurrentHealth`) (* (`local.Damage`) 2.0)))))
  (if (<= _output_get_2 0.0)
    (bind _output_get_3 (set `self.IsDead` true))
    (`self.Death`)
    (return _output_get_3)
    (else
      (`KismetSystemLibrary.PrintString` (`KismetStringLibrary.Conv_DoubleToString` (`self.CurrentHealth`)))
      (return false))))

(fn `UpdateMaxLife`
  (set `self.MaxHealth` (* (`self.MaxHealth`) 1.2)))