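; BPC_Score is an actor component that tracks the player's score from combat results.
; On BeginPlay it caches the first-person player character.
; AddScore picks a fixed value by priority (kill, then headshot, then plain hit), adds it to the running score and passes it to the player's main HUD.
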(event `self.ReceiveBeginPlay`
  (bind _asbp_first_person_character (cast `/Game/BP_/BP_Player/BP_FirstPersonCharacter` (`GameplayStatics.GetPlayerCharacter` 0)))
  (set `self.Player` _asbp_first_person_character))

(fn `AddScore`
  (params (Dead :type Boolean) (Head :type Boolean) (Hit :type Boolean))
  (locals (Value :type Integer))
  (if Dead
    (set `local.Value` 50)
    (set `self.Score` (+ (`local.Value`) (`self.Score`)) :!label _label)
    (`/Game/BP_/Widgets/WB_MainHUD.AddScore` (`/Game/BP_/BP_Player/BP_FirstPersonCharacter.MainHUD` (`self.Player`)) (`local.Value`))
    (elif Head
      (set `local.Value` 15)
      (goto _label)
      (elif Hit
        (set `local.Value` 10)
        (goto _label)))))