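; Buff pedestal actor that offers the player a choice of stat upgrades through an on-screen menu.
; BeginPlay creates a hidden buff HUD and binds each button's choose event.
; Capsule overlap toggles the menu and mouse input; choosing upgrades the character's stats, fires a buff-chosen dispatcher and sets BuffChosen to false, leaving the menu re-openable.
; Appear and disappear events raise or lower the pedestal with MoveComponentTo.
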(event `self.ReceiveBeginPlay`
  (bind _returnvalue (`|CreateWidget` "/Game/BP_/Widgets/BuffHUD/WB_MainBuffHUD.WB_MainBuffHUD_C"))
  (bind _output_get (set `self.BuffHUD` _returnvalue))
  (`UserWidget.AddToViewport` _output_get 100)
  (`Widget.SetVisibility` _output_get "Hidden")
  (bind _asbp_first_person_character (cast `/Game/FirstPerson/BP_Player/BP_FirstPersonCharacter` (`GameplayStatics.GetPlayerCharacter` 0)))
  (set `self.PlayerCharacter` _asbp_first_person_character)
  (for _array_element (`PanelWidget.GetAllChildren` (`/Game/BP_/Widgets/BuffHUD/WB_MainBuffHUD.BuffList` (`self.BuffHUD`)))
    (bind _aswb_buff_button (cast `/Game/BP_/Widgets/BuffHUD/WB_BuffButton` _array_element))
    (`KismetArrayLibrary.Array_Add` (`self.BuffButtons`) _aswb_buff_button)
    (add `/Game/BP_/Widgets/BuffHUD/WB_BuffButton.ED_ChooseBuff` _aswb_buff_button (delegate `ED_ChooseBuff_Event`))))

(event `ED_ChooseBuff_Event`
  (params (Buff :type "/Game/BP_/Buff/BuffData Structure"))
  (bind _returnvalue (`GameplayStatics.GetPlayerController` 0))
  (set `self.BuffChosen` false)
  (`Widget.SetVisibility` (`self.BuffHUD`) "Hidden")
  (`/Game/FirstPerson/BP_Player/BP_FirstPersonCharacter.Upgrade Stats` (`self.PlayerCharacter`) Buff_Stats_14_94E66CD74699D2B2B0BB3F88C853FC06)
  (`self.ED_BuffChosen` (struct))
  (set `PlayerController.bShowMouseCursor` false _returnvalue)
  (`WidgetBlueprintLibrary.SetInputMode_GameOnly` _returnvalue))

(event `self.Capsule.OnComponentBeginOverlap`
  (params (OverlappedComponent :type "PrimitiveComponent Object Reference") (OtherActor :type "Actor Object Reference") (OtherComp :type "PrimitiveComponent Object Reference") (OtherBodyIndex :type Integer) (bFromSweep :type Boolean) (SweepResult :type "HitResult Structure (by ref)"))
  (bind _returnvalue (`GameplayStatics.GetPlayerController` 0))
  (if (not (`self.BuffChosen`))
    (`Widget.SetVisibility` (`self.BuffHUD`) "Visible")
    (set `PlayerController.bShowMouseCursor` true _returnvalue)
    (`WidgetBlueprintLibrary.SetInputMode_GameAndUIEx` _returnvalue null)))

(event `self.Capsule.OnComponentEndOverlap`
  (params (OverlappedComponent :type "PrimitiveComponent Object Reference") (OtherActor :type "Actor Object Reference") (OtherComp :type "PrimitiveComponent Object Reference") (OtherBodyIndex :type Integer))
  (bind _returnvalue (`GameplayStatics.GetPlayerController` 0))
  (`Widget.SetVisibility` (`self.BuffHUD`) "Hidden")
  (set `PlayerController.bShowMouseCursor` false _returnvalue)
  (`WidgetBlueprintLibrary.SetInputMode_GameOnly` _returnvalue))

(event `CE_Apear`
  (bind _transform (`self.Transform`))
  (bind (_relativelocation_x _relativelocation_y _relativelocation_z) (`KismetMathLibrary.BreakVector` (`SceneComponent.RelativeLocation` _transform)))
  (`KismetSystemLibrary.MoveComponentTo` _transform (`KismetMathLibrary.MakeVector` _relativelocation_x _relativelocation_y (+ _relativelocation_z 600.0))))

(event `CE_Disapear`
  (bind _transform (`self.Transform`))
  (bind (_relativelocation_x _relativelocation_y _relativelocation_z) (`KismetMathLibrary.BreakVector` (`SceneComponent.RelativeLocation` _transform)))
  (`KismetSystemLibrary.MoveComponentTo` _transform (`KismetMathLibrary.MakeVector` _relativelocation_x _relativelocation_y (- _relativelocation_z 600.0))))

(fn `UserConstructionScript`)