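; Object pool actor that pre-spawns BP_EnemyMinionsSimon enemies at BeginPlay and recycles them through their destroy dispatcher.
; Pooled enemies are moved to the pool, attached, hidden, stripped of collision and unpossessed by their AI controller.
; RequestEnemy grows the pool when empty, then detaches and returns the first enemy with collision, visibility and default controller restored.
; Its EnemyType input is unused, so only that one class is served.
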(event `self.ReceiveBeginPlay`
  (for _ (range (+ (`self.BaseEnemyNumber`) 1))
    (`self.CE_IncreasePoolCount`)))

(event `CE_IncreasePoolCount`
  (bind _returnvalue (`|SpawnActorFromClass` "/Game/BP_/Enemy/BP_EnemyMinionsSimon.BP_EnemyMinionsSimon_C" (`KismetMathLibrary.MakeTransform` (0.0 0.0 0.0)) "AlwaysSpawn" "MultiplyWithRoot" null null))
  (`self.PutInPool` _returnvalue)
  (add `/Game/BP_/Enemy/BP_EnemyMinionsSimon.ED_OnDestroy` _returnvalue (delegate `CE_ReturnToPool`)))

(event `CE_ReturnToPool`
  (params (Enemy :type "/Game/BP_/Enemy/BP_EnemyMinionsSimon Object Reference"))
  (`self.PutInPool` Enemy))

(fn `PutInPool`
  (params (Enemy :type "/Game/BP_/Enemy/BP_EnemyMinionsSimon Object Reference"))
  (bind _enemy (`local.Enemy`))
  (`self.K2_SetActorLocation` Enemy (`self.K2_GetActorLocation`) false false)
  (`PrimitiveComponent.SetCollisionEnabled` (`Character.Mesh` (`local.Enemy`)) "NoCollision")
  (`PrimitiveComponent.SetCollisionEnabled` (`/Game/BP_/Enemy/BP_EnemyMinions.Cube` (`local.Enemy`)) "NoCollision")
  (`self.K2_AttachToActor` (`local.Enemy`) self "None" "KeepWorld" "KeepWorld" "KeepWorld" true)
  (`self.SetActorHiddenInGame` _enemy true)
  (`Controller.UnPossess` (`AIBlueprintHelperLibrary.GetAIController` _enemy))
  (`KismetArrayLibrary.Array_Add` (`self.EnemyPool`) (`local.Enemy`)))

(fn `RequestEnemy`
  (params (EnemyType :type Boolean))
  (returns (Enemy :type "/Game/BP_/Enemy/BP_EnemyMinionsSimon Object Reference"))
  (locals (SelectedEnemy :type "/Game/BP_/Enemy/BP_EnemyMinionsSimon Object Reference"))
  (bind _output (`|GetArrayItem` (`self.EnemyPool`)))
  (if (not (> (`KismetArrayLibrary.Array_Length` (`self.EnemyPool`)) 0))
    (`self.CE_IncreasePoolCount`))
  (`/Engine/EditorBlueprintResources/StandardMacros.IsValid` _output
    (:`Is Valid`
      (bind _output_get (set `local.SelectedEnemy` _output))
      (`KismetArrayLibrary.Array_Remove` (`self.EnemyPool`))
      (`self.K2_DetachFromActor` _output_get "KeepWorld" "KeepWorld" "KeepWorld")
      (`PrimitiveComponent.SetCollisionEnabled` (`Character.Mesh` _output_get) "QueryAndPhysics")
      (`PrimitiveComponent.SetCollisionEnabled` (`/Game/BP_/Enemy/BP_EnemyMinions.Cube` _output_get) "QueryAndPhysics")
      (`self.SetActorHiddenInGame` _output_get false)
      (`Pawn.SpawnDefaultController` _output_get)
      (return _output_get))))

(fn `UserConstructionScript`)