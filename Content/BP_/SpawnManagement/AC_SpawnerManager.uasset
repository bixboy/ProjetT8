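; AC_SpawnerManager is a spawner manager that runs the enemy spawning for each battle wave.
; It gathers every BP_Spawner in the level at BeginPlay and takes the enemy count from wave data when a battle starts.
; After an initial delay, a self-calling timed event triggers a random spawner per enemy until the count runs out, then calls the all-enemies-spawned dispatcher.
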(event `self.ReceiveBeginPlay`
  (bind _outactors (`GameplayStatics.GetAllActorsOfClass` "/Game/BP_/SpawnManagement/BP_Spawner.BP_Spawner_C"))
  (set `self.Spawners` _outactors))

(event `CE_StartBattle`
  (params (`Wave Data` :type "/Game/BP_/WaveManagement/WaveData Structure"))
  (set `self.EnemyRemaining` `Wave Data_EnemyNb_2_B5E666B44196707641F95E902C7D6B1C`)
  (`KismetSystemLibrary.Delay` 5.0)
  (set `self.SpawnDelay` 1.0)
  (`self.CE_Spawning`))

(event `CE_Spawning`
  (`KismetSystemLibrary.Delay` (`self.SpawnDelay`))
  (if (> (`self.EnemyRemaining`) 0)
    (`/Game/BP_/SpawnManagement/BP_Spawner.Spawn` (`KismetArrayLibrary.Array_Random` (`self.Spawners`)) false)
    (`/Engine/EditorBlueprintResources/StandardMacros.DecrementInt` (`self.EnemyRemaining`)
      (:`  `
        (`self.CE_Spawning`)))
    (else
      (`self.ED_AllEnemySpawned`))))