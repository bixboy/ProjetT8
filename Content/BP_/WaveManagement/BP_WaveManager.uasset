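; BP_WaveManager runs the wave loop, tracking the wave number and starting each battle through SpawnerManager.
; On BeginPlay it reads the current wave's data, passes it to the spawner and broadcasts start-battle and begin-wave dispatchers.
; Ending a wave broadcasts, increments the number and immediately initializes the next.
; A separate buff-choice event broadcasts its own dispatcher, but BuffAppear and ReadData are empty stubs.
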(event `self.ReceiveBeginPlay`
  (`self.CE_InitWave`))

(event `CE_InitWave`
  (bind _wavedata (`self.ReadData` (`self.WaveNb`)))
  (`self.CE_StartBattle` _wavedata)
  (`self.ED_BeginWave`))

(event `CE_StartBattle`
  (params (WaveData :type "/Game/BP_/WaveManagement/WaveData Structure"))
  (`/Game/BP_/SpawnManagement/AC_SpawnerManager.CE_StartBattle` (`self.SpawnerManager`) WaveData)
  (`self.ED_StartBattle` WaveData))

(event `CE_StartBuffChoice`
  (`self.BuffAppear`)
  (`self.ED_StartBuffChoice`))

(event `CE_EndWave`
  (`self.ED_EndWave`)
  (set `self.WaveNb` (+ (`self.WaveNb`) 1))
  (`self.CE_InitWave`))

(fn `BuffAppear`)

(fn `ReadData`
  (params (`Wave Count` :type Integer))
  (returns (WaveData :type "/Game/BP_/WaveManagement/WaveData Structure"))
  (return))

(fn `UserConstructionScript`)