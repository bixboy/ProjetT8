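; Actor component that shows the live enemy count on screen and detects the end of a battle.
; On BeginPlay it creates the counter widget and binds to the all-enemies-spawned event on the WaveManager's SpawnerManager.
; Tick polls EnemyCount to refresh the text; once spawning has finished and the count empties, it hides the widget and starts the WaveManager's buff choice, using a flag to fire once per battle.
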(event `self.ReceiveBeginPlay`
  (bind _returnvalue (`|CreateWidget` "/Game/BP_/Widgets/WaveHUD/WB_EnemyCounter.WB_EnemyCounter_C"))
  (bind _output_get (set `self.Widget` _returnvalue))
  (`UserWidget.AddToViewport` _output_get 0)
  (bind _returnvalue_2 (`GameplayStatics.GetActorOfClass` "/Game/BP_/WaveManagement/BP_WaveManager.BP_WaveManager_C"))
  (bind _output_get_2 (set `self.WaveManager` _returnvalue_2))
  (set `self.NoEnemyRemaining` false)
  (add `/Game/BP_/Manager/SpawnManagement/AC_SpawnerManager.ED_AllEnemySpawned` (`/Game/BP_/WaveManagement/BP_WaveManager.SpawnerManager` _output_get_2) (delegate `ED_AllEnemySpawned_Event`))
  (set `TextBlock.Text` (`KismetTextLibrary.Conv_IntToText` (`self.EnemyCount`)) (`/Game/BP_/Widgets/WaveHUD/WB_EnemyCounter.enemyCounter` (`self.Widget`))))

(event `ED_AllEnemySpawned_Event`
  (set `self.NoEnemyRemaining` true))

(event `self.ReceiveTick`
  (params (DeltaSeconds :type "Float (single-precision)"))
  (if (> (`self.EnemyCount`) 0)
    (`Widget.SetVisibility` (`self.Widget`) "Visible")
    (set `TextBlock.Text` (`KismetTextLibrary.Conv_IntToText` (`self.EnemyCount`)) (`/Game/BP_/Widgets/WaveHUD/WB_EnemyCounter.enemyCounter` (`self.Widget`)))
    (set `self.InitEndBattle` true)
    (elif (`self.NoEnemyRemaining`)
      (if (`self.InitEndBattle`)
        (`Widget.SetVisibility` (`self.Widget`) "Hidden")
        (set `self.InitEndBattle` false)
        (`/Game/BP_/WaveManagement/BP_WaveManager.CE_StartBuffChoice` (`self.WaveManager`))))))