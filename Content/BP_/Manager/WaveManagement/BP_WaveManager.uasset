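; BP_WaveManager runs the wave loop, alternating battles with a buff choice at a pedestal.
; Each wave reads its row from WaveDataTable by wave number and passes it to SpawnerManager, broadcasting phase changes through event dispatchers.
; CE_StartBuffChoice, not called internally, fills the pedestal's buttons with random BuffDataTable rows, possibly repeated, and reveals it.
; The pedestal's buff-chosen event hides it, increments the wave and starts the next.
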(event `self.ReceiveBeginPlay`
  (`self.CE_InitWave`)
  (bind _returnvalue (`GameplayStatics.GetActorOfClass` "/Game/BP_/Buff/BP_Pedestal.BP_Pedestal_C"))
  (bind _output_get (set `self.Pedestal` _returnvalue))
  (add `/Game/BP_/Buff/BP_Pedestal.ED_BuffChosen` _output_get (delegate `ED_BuffChosen_Event`)))

(event `ED_BuffChosen_Event`
  (params (Buff :type "/Game/BP_/Buff/BuffData Structure"))
  (`self.CE_EndWave`))

(event `CE_InitWave`
  (bind _wavedata (`self.ReadData` (`self.WaveNb`)))
  (`self.CE_StartBattle` _wavedata)
  (`self.ED_BeginWave`))

(event `CE_StartBattle`
  (params (WaveData :type "/Game/BP_/Manager/WaveManagement/WaveData Structure"))
  (`/Game/BP_/Manager/SpawnManagement/AC_SpawnerManager.CE_StartBattle` (`self.SpawnerManager`) WaveData)
  (`self.ED_StartBattle` WaveData))

(event `CE_StartBuffChoice`
  (`self.BuffAppear`)
  (`self.ED_StartBuffChoice`)
  (`KismetSystemLibrary.PrintString` "BuffCHoice"))

(event `CE_EndWave`
  (`/Game/BP_/Buff/BP_Pedestal.CE_Disapear` (`self.Pedestal`))
  (`self.ED_EndWave`)
  (`/Engine/EditorBlueprintResources/StandardMacros.IncrementInt` (`self.WaveNb`)
    (:`  `
      (`self.CE_InitWave`))))

(fn `BuffAppear`
  (bind _pedestal (`self.Pedestal`))
  (for _array_element (`/Game/BP_/Buff/BP_Pedestal.BuffButtons` _pedestal)
    (bind _outrownames (`DataTableFunctionLibrary.GetDataTableRowNames` "/Game/BP_/Buff/BuffDataTable.BuffDataTable"))
    (bind _returnvalue (`|GetDataTableRow` "/Game/BP_/Buff/BuffDataTable.BuffDataTable" (`|GetArrayItem` _outrownames (`KismetMathLibrary.RandomInteger` (`KismetArrayLibrary.Array_Length` _outrownames))))
      (:`then`
        (`/Game/BP_/Widgets/BuffHUD/WB_BuffButton.CE_SetBuff` _array_element _returnvalue))))
  (`/Game/BP_/Buff/BP_Pedestal.CE_Apear` _pedestal))

(fn `ReadData`
  (params (`Wave Count` :type Integer))
  (returns (WaveData :type "/Game/BP_/Manager/WaveManagement/WaveData Structure"))
  (bind _outrownames (`DataTableFunctionLibrary.GetDataTableRowNames` "/Game/BP_/Manager/WaveManagement/WaveDataTable.WaveDataTable"))
  (bind _returnvalue (`|GetDataTableRow` "/Game/BP_/Manager/WaveManagement/WaveDataTable.WaveDataTable" (`|GetArrayItem` _outrownames (- `Wave Count` 1)))
    (:`then`
      (return _returnvalue))))

(fn `UserConstructionScript`)